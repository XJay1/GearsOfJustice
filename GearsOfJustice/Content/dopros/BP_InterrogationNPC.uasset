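; BP_InterrogationNPC is an NPC the player can approach to trigger an interrogation.
; Its Sphere overlap detects the player's pawn, enables input, sets a proximity flag and shows an interaction prompt widget with the NPC's text.
; The Interact event calls DoprosSpawn on DoprosComponent while the player is nearby.
; Ending overlap clears the flag and hides the prompt, without checking the actor or disabling input.
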(event `self.Sphere.OnComponentBeginOverlap`
  (params (OverlappedComponent :type "PrimitiveComponent Object Reference") (OtherActor :type "Actor Object Reference") (OtherComp :type "PrimitiveComponent Object Reference") (OtherBodyIndex :type Integer) (bFromSweep :type Boolean) (SweepResult :type "HitResult Structure (by ref)"))
  (bind _returnvalue (`GameplayStatics.GetPlayerController` 0))
  (bind _widget (`self.Widget`))
  (bind _w_interact (`self.W_Interact`))
  ;[1 1 1] проверка на игрока
  (if (== OtherActor (`Controller.K2_GetPawn` _returnvalue))
    (`self.EnableInput` _returnvalue)
    (bind _output_get (set `self.Is Player Nearby` true))
    (set `/Game/MiniGames/W_Interact.InteractText` (`self.Interact Text`) _w_interact)
    (`WidgetComponent.SetWidget` _widget _w_interact)
    (`SceneComponent.SetVisibility` _widget _output_get false)))

(event `/Game/dopros/BPI_interface.Interact`
  ;[1 1 1] проверка на игрока
  (if (`self.Is Player Nearby`)
    (`/Game/dopros/Dopros_component.Dopros_Spawn` (`self.Dopros_component`))))

(event `self.Sphere.OnComponentEndOverlap`
  (params (OverlappedComponent :type "PrimitiveComponent Object Reference") (OtherActor :type "Actor Object Reference") (OtherComp :type "PrimitiveComponent Object Reference") (OtherBodyIndex :type Integer))
  ;[1 1 1] проверка на игрока
  (bind _output_get (set `self.Is Player Nearby` false))
  (`SceneComponent.SetVisibility` (`self.Widget`) _output_get false))

(fn `UserConstructionScript`)