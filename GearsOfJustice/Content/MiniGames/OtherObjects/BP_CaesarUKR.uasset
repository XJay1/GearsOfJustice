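; BP_CaesarUKR is a minigame actor that applies a Caesar cipher to InputText, apparently for the Ukrainian alphabet.
; It runs two seconds after BeginPlay and on every Box overlap, which also enables player input.
; Each character found in AlphabetString moves by Shift, wrapping within its own 33-character half, while other characters pass through unchanged.
; The input and resulting EncryptedText are only shown via PrintString.
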(event `self.ReceiveBeginPlay`
  (`KismetSystemLibrary.K2_SetTimerDelegate` (delegate `Caesar`) 2.0))

(event `Caesar`
  (bind _inputtext (`self.InputText`))
  (set `self.EncryptedText` "" :!label _label)
  (`KismetSystemLibrary.PrintString` (`KismetStringLibrary.Concat_StrStr` "ВВОД: " _inputtext))
  (for _array_element (`KismetStringLibrary.GetCharacterArrayFromString` _inputtext)
    (bind _returnvalue (`KismetStringLibrary.FindSubstring` (`self.AlphabetString`) _array_element))
    (if (== _returnvalue -1)
      (set `self.EncryptedText` (`KismetStringLibrary.Concat_StrStr` (`self.EncryptedText`) _array_element))
      (elif (>= _returnvalue 33)
        (bind _returnvalue_2 (+ _returnvalue (`self.Shift`)))
        (if (< _returnvalue_2 33)
          (set `self.EncryptedText` (`KismetStringLibrary.Concat_StrStr` (`self.EncryptedText`) (`KismetStringLibrary.Mid` (`self.AlphabetString`) (+ _returnvalue_2 33) 1)) :!label _label_2)
          (elif (>= _returnvalue_2 66)
            (set `self.EncryptedText` (`KismetStringLibrary.Concat_StrStr` (`self.EncryptedText`) (`KismetStringLibrary.Mid` (`self.AlphabetString`) (- _returnvalue_2 33) 1)) :!label _label_3)
            (else
              (set `self.EncryptedText` (`KismetStringLibrary.Concat_StrStr` (`self.EncryptedText`) (`KismetStringLibrary.Mid` (`self.AlphabetString`) _returnvalue_2 1)) :!label _label_4))))
        (elif (< _returnvalue_2 0)
          (goto _label_2)
          (elif (>= _returnvalue_2 33)
            (goto _label_3)
            (else
              (goto _label_4)))))))
  (`KismetSystemLibrary.PrintString` (`KismetStringLibrary.Concat_StrStr` "ВЫВОД: " (`self.EncryptedText`))))

(event `self.Box.OnComponentBeginOverlap`
  (params (OverlappedComponent :type "PrimitiveComponent Object Reference") (OtherActor :type "Actor Object Reference") (OtherComp :type "PrimitiveComponent Object Reference") (OtherBodyIndex :type Integer) (bFromSweep :type Boolean) (SweepResult :type "HitResult Structure (by ref)"))
  (`self.EnableInput` (`GameplayStatics.GetPlayerController` 0))
  (goto _label))

(fn `UserConstructionScript`)