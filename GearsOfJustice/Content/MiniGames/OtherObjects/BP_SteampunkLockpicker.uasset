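; BP_SteampunkLockpicker is a steampunk lockpicker pickup that the player collects as a clue by pressing E in range.
; It destroys itself on BeginPlay if the GameInstance interact check for its Type fails, and a sphere overlap toggles the prompt widget.
; Pickup shows a notification, updates GameInstance clue and interact state, then destroys the actor.
; SetVisible enables custom depth; AddEvidence, uncalled here, appends an interrogation evidence entry.
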(event `SetVisible`
  (`PrimitiveComponent.SetRenderCustomDepth` (`self.SteampunkLPFull`) true))

(event `self.ReceiveBeginPlay`
  (bind _takebool (message `/Game/MiniGames/BPI_MiniGameInteract.GetInteract` (`GameplayStatics.GetGameInstance`) (`self.Type`)))
  (if (not _takebool)
    (`self.K2_DestroyActor`)))

(event `self.Sphere.OnComponentBeginOverlap`
  (params (OverlappedComponent :type "PrimitiveComponent Object Reference") (OtherActor :type "Actor Object Reference") (OtherComp :type "PrimitiveComponent Object Reference") (OtherBodyIndex :type Integer) (bFromSweep :type Boolean) (SweepResult :type "HitResult Structure (by ref)"))
  (bind _returnvalue (`GameplayStatics.GetPlayerController` 0))
  (bind _w_interact (`self.W_Interact`))
  (bind _widget (`self.Widget`))
  (if (== OtherActor (`Controller.K2_GetPawn` _returnvalue))
    (`self.EnableInput` _returnvalue)
    (bind _output_get (set `self.bIsPlayerInRange` true))
    (set `/Game/MiniGames/W_Interact.InteractText` (`self.Interact Text`) _w_interact)
    (`WidgetComponent.SetWidget` _widget _w_interact)
    (`SceneComponent.SetVisibility` _widget _output_get false)))

(event `self.Sphere.OnComponentEndOverlap`
  (params (OverlappedComponent :type "PrimitiveComponent Object Reference") (OtherActor :type "Actor Object Reference") (OtherComp :type "PrimitiveComponent Object Reference") (OtherBodyIndex :type Integer))
  (bind _output_get (set `self.bIsPlayerInRange` false))
  (`SceneComponent.SetVisibility` (`self.Widget`) _output_get false))

(event `Key|E` :consume false
  (params (Key :type "Key Structure"))
  (bind _returnvalue (`GameplayStatics.GetGameInstance`))
  (bind _w_notification (`self.W_Notification`))
  (:`Pressed`
    (if (`self.bIsPlayerInRange`)
      (`UserWidget.AddToViewport` _w_notification 2)
      (`/Game/MiniGames/OtherObjects/W_Notification.NotificationSteampunkLP` _w_notification)
      (set `self.bIsPlayerInRange` false)
      (message `/Game/CluesDataBase/BPI_Clues.MarkClueAsFound` _returnvalue "SteampunkLockpicker")
      (message `/Game/MiniGames/BPI_MiniGameInteract.CanInteract` _returnvalue (`self.Type`))
      (`self.K2_DestroyActor`))))

(fn `AddEvidence`
  (bind _asbp_game_instance (cast `/Game/GameInstance/BP_GameInstance` (`GameplayStatics.GetGameInstance`)))
  (`KismetArrayLibrary.Array_Add` (`/Game/GameInstance/BP_GameInstance.Dopros_evidence` _asbp_game_instance) (make `/Game/dopros/Round_info` (`KismetMathLibrary.Conv_IntToInt64` (`/Game/GameInstance/BP_GameInstance.ID+` _asbp_game_instance)) "NewEnumerator1" "NewEnumerator1" "Дивний механізм Рене Бельєр" null))
  (set `/Game/GameInstance/BP_GameInstance.ID+` (+ (`/Game/GameInstance/BP_GameInstance.ID+` _asbp_game_instance) 1) _asbp_game_instance))

(fn `UserConstructionScript`)