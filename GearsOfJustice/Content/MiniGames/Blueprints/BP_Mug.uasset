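; BP_Mug is an interactable mug actor that starts the fingerprint analyzer minigame.
; Its MugBox overlap with a BP_GOJBaseCharacter sets an in-range flag, if interactable, and shows a text prompt that hides when the character leaves.
; The actor enables player 0 input itself, so pressing E in range spawns BP_FingerprintAnalyzer at a hardcoded world location, calls StartMinigame and hides the prompt.
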(event `self.ReceiveBeginPlay`
  (`self.EnableInput` (`GameplayStatics.GetPlayerController` 0)))

(event `self.MugBox.OnComponentBeginOverlap`
  (params (OverlappedComponent :type "PrimitiveComponent Object Reference") (OtherActor :type "Actor Object Reference") (OtherComp :type "PrimitiveComponent Object Reference") (OtherBodyIndex :type Integer) (bFromSweep :type Boolean) (SweepResult :type "HitResult Structure (by ref)"))
  ;[0.4417 0.4498 1] Надпись
  (cast `/Game/Player/BP_GOJBaseCharacter` OtherActor)
  (if (`self.bIsInteractable`)
    (bind _output_get (set `self.bIsPlayerInRange` true))
    (`SceneComponent.SetVisibility` (`self.TextRender`) _output_get false)))

(event `self.MugBox.OnComponentEndOverlap`
  (params (OverlappedComponent :type "PrimitiveComponent Object Reference") (OtherActor :type "Actor Object Reference") (OtherComp :type "PrimitiveComponent Object Reference") (OtherBodyIndex :type Integer))
  ;[0.4417 0.4498 1] Надпись
  (cast `/Game/Player/BP_GOJBaseCharacter` OtherActor)
  (bind _output_get (set `self.bIsPlayerInRange` false))
  (`SceneComponent.SetVisibility` (`self.TextRender`) _output_get false))

(event `Key|E`
  (params (Key :type "Key Structure"))
  ;[0.6615 0.6615 0.6615] Взаимодействие для начала мини игры
  (:`Pressed`
    (if (`self.bIsPlayerInRange`)
      (bind _returnvalue (`|SpawnActorFromClass` "/Game/MiniGames/Blueprints/BP_FingerprintAnalyzer.BP_FingerprintAnalyzer_C" (`KismetMathLibrary.MakeTransform` (1076.0 3228.0 161.0)) "Undefined" "MultiplyWithRoot" null null))
      (`/Game/MiniGames/Blueprints/BP_FingerprintAnalyzer.Start mini-game` _returnvalue)
      (`SceneComponent.SetVisibility` (`self.TextRender`) false false))))

(fn `UserConstructionScript`)