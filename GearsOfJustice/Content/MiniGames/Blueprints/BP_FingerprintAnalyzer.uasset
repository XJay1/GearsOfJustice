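; BP_FingerprintAnalyzer is the actor that runs a fingerprint analysis mini-game on a mug.
; Starting it shows the UIFingerprintGame widget, switches to the minigame camera and enables the cursor, with right-mouse drag yawing the mug.
; Clicking collision components uses their first component tag to look up a fingerprint in a dictionary and send it to the widget.
; Ending prints the result (evidence saving is only a placeholder), restores game input, makes BP_Mug non-interactable and destroys itself.
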(event `Start mini-game`
  (bind _returnvalue (`GameplayStatics.GetPlayerController` 0))
  ;[0.3847 0.5209 1] Старт мини-игры
  (`self.EnableInput` _returnvalue)
  (bind _returnvalue_2 (`|CreateWidget` (`self.UI_FingerprintGame`)))
  (bind _output_get (set `self.FingerprintGameUI` _returnvalue_2))
  (`/Game/MiniGames/UI/UI_FingerprintGame.InitializeDossierItems` _output_get)
  (`UserWidget.AddToViewport` _output_get 0)
  (`PlayerController.SetViewTargetWithBlend` _returnvalue (`ActorComponent.GetOwner` (`self.MinigameCamera`)) 0.0 "VTBlend_Linear" 0.0 false)
  (set `PlayerController.bShowMouseCursor` true _returnvalue)
  (set `PlayerController.bEnableMouseOverEvents` true _returnvalue)
  (`WidgetBlueprintLibrary.SetInputMode_GameAndUIEx` _returnvalue (`self.FingerprintGameUI`)))

(event `self.ReceiveBeginPlay`)

(event `Key|E`
  (params (Key :type "Key Structure"))
  ;[0 0 0] Заглушка от багов
  (:`Pressed`
    (if false
      (`KismetSystemLibrary.PrintString` "Hello"))))

(event `End Mini-game`
  (params (IsSuccessful :type Boolean))
  (bind _returnvalue (`GameplayStatics.GetPlayerController` 0))
  ;[1 0.3759 0.3261] Завершение мини игры
  (if IsSuccessful
    (`KismetSystemLibrary.PrintString` "Будет сохранение улики")
    (else
      (`KismetSystemLibrary.PrintString` "Мини игра провалена")))
  (`KismetSystemLibrary.Delay` 2.0)
  (`Widget.RemoveFromParent` (`self.FingerprintGameUI`))
  (set `PlayerController.bShowMouseCursor` false _returnvalue)
  (set `PlayerController.bEnableMouseOverEvents` false _returnvalue)
  (`WidgetBlueprintLibrary.SetInputMode_GameOnly` _returnvalue)
  (bind _outactors (`GameplayStatics.GetAllActorsOfClass` "/Game/MiniGames/Blueprints/BP_Mug.BP_Mug_C"))
  (set `/Game/MiniGames/Blueprints/BP_Mug.bIsInteractable` false (`|GetArrayItem` _outactors))
  (`self.K2_DestroyActor`))

(event `self.collision5.OnClicked`
  (params (TouchedComponent :type "PrimitiveComponent Object Reference") (ButtonPressed :type "Key Structure"))
  (bind _hoveredfingerprinttag (`self.HoveredFingerprintTag`))
  (bind _fingerprintgameui (`self.FingerprintGameUI`))
  ;[0.5657 1 0.9602] Выбор тега из взаимодействия с коллизией
  (`self.Hovered Tag` TouchedComponent)
  ;[0.3844 1 0.2667] Выбор отпечатка по его тегу
  (if (!= _hoveredfingerprinttag "None") :!label _label
    (set `self.SelectedFingerprint` (`BlueprintMapLibrary.Map_Find` (`self.FingerprintDictionary`) _hoveredfingerprinttag))
    (if (`KismetSystemLibrary.IsValid` _fingerprintgameui)
      (`/Game/MiniGames/UI/UI_FingerprintGame.UpdateSelectedFingerprint` _fingerprintgameui (`self.SelectedFingerprint`)))))

(event `InputAxis|RotateCup`
  (params (AxisValue :type "Float (single-precision)"))
  ;[1 0.7962 0.3395] Кручение кружки
  (if (`self.bIsDraggingCup`)
    (`SceneComponent.K2_AddRelativeRotation` (`self.mug`) (`KismetMathLibrary.MakeRotator` 0.0 0.0 (* AxisValue 3.0)) false false)))

(event `self.collision2.OnClicked`
  (params (TouchedComponent :type "PrimitiveComponent Object Reference") (ButtonPressed :type "Key Structure"))
  ;[0.5657 1 0.9602] Выбор тега из взаимодействия с коллизией
  (`self.Hovered Tag` TouchedComponent)
  (goto _label))

(event `self.collision1.OnClicked`
  (params (TouchedComponent :type "PrimitiveComponent Object Reference") (ButtonPressed :type "Key Structure"))
  ;[0.5657 1 0.9602] Выбор тега из взаимодействия с коллизией
  (`self.Hovered Tag` TouchedComponent)
  (goto _label))

(event `Key|RightMouseButton`
  (params (Key :type "Key Structure"))
  ;[1 0.7962 0.3395] Кручение кружки
  (:`Pressed`
    (set `self.bIsDraggingCup` true))
  (:`Released`
    (set `self.bIsDraggingCup` false)))

(event `self.collision3.OnClicked`
  (params (TouchedComponent :type "PrimitiveComponent Object Reference") (ButtonPressed :type "Key Structure"))
  ;[0.5657 1 0.9602] Выбор тега из взаимодействия с коллизией
  (`self.Hovered Tag` TouchedComponent)
  (goto _label))

(event `self.collision4_t.OnClicked`
  (params (TouchedComponent :type "PrimitiveComponent Object Reference") (ButtonPressed :type "Key Structure"))
  ;[0.5657 1 0.9602] Выбор тега из взаимодействия с коллизией
  (`self.Hovered Tag` TouchedComponent)
  (goto _label))

(fn `Hovered Tag`
  (params (tag :type "ActorComponent Object Reference"))
  (set `self.HoveredFingerprintTag` (`|GetArrayItem` (`ActorComponent.ComponentTags` tag))))

(fn `UserConstructionScript`)