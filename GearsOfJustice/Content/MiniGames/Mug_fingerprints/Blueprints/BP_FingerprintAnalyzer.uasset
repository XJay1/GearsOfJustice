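; Fingerprint mini-game actor: the player rotates a mug, dusts it for prints and picks one to compare in the game UI.
; Pressing E traces from the cursor, spawns a powder effect and moves a detection sphere whose box overlaps reveal decals and enable their click colliders.
; Clicked colliders' tags look up fingerprints for the widget.
; Success adds interrogation evidence; ending or giving up restores lighting, camera and input, then destroys the actor.
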(event `self.BoxOverlap1.OnComponentBeginOverlap`
  (params (OverlappedComponent :type "PrimitiveComponent Object Reference") (OtherActor :type "Actor Object Reference") (OtherComp :type "PrimitiveComponent Object Reference") (OtherBodyIndex :type Integer) (bFromSweep :type Boolean) (SweepResult :type "HitResult Structure (by ref)"))
  ;[0.7721 0.4346 1] Активация и раскраска отпечатков
  (if (== OtherComp (`self.DetectionSphere`))
    (`SceneComponent.SetVisibility` (`self.Decal_Fingerprint1`) true false)
    (`PrimitiveComponent.SetCollisionEnabled` (`self.collision1`) "QueryAndPhysics")))

(event `self.BPC_Pause.UnPauseGame`
  (`WidgetBlueprintLibrary.SetInputMode_GameAndUIEx` (`GameplayStatics.GetPlayerController` 0) (`self.FingerprintGameUI`)))

(event `self.BoxOverlap2.OnComponentBeginOverlap`
  (params (OverlappedComponent :type "PrimitiveComponent Object Reference") (OtherActor :type "Actor Object Reference") (OtherComp :type "PrimitiveComponent Object Reference") (OtherBodyIndex :type Integer) (bFromSweep :type Boolean) (SweepResult :type "HitResult Structure (by ref)"))
  ;[0.7721 0.4346 1] Активация и раскраска отпечатков
  (if (== OtherComp (`self.DetectionSphere`))
    (`SceneComponent.SetVisibility` (`self.Decal_Fingerprint2`) true false)
    (`PrimitiveComponent.SetCollisionEnabled` (`self.collision2`) "QueryAndPhysics")))

(event `self.BPC_Pause.PauseGame`
  (params (PauseWidget :type "/Game/Menu/Blueprint/W_PauseMenu Object Reference"))
  (set `/Game/Menu/Blueprint/W_PauseMenu.NameActivities` "Fingerprint" PauseWidget)
  (`Widget.SetVisibility` (`/Game/Menu/Blueprint/W_PauseMenu.SaveButton` PauseWidget) "Collapsed")
  (set `/Game/Menu/Blueprint/W_PauseMenu.BPC_Pause` (`self.BPC_Pause`) PauseWidget))

(event `self.BoxOverlap3.OnComponentBeginOverlap`
  (params (OverlappedComponent :type "PrimitiveComponent Object Reference") (OtherActor :type "Actor Object Reference") (OtherComp :type "PrimitiveComponent Object Reference") (OtherBodyIndex :type Integer) (bFromSweep :type Boolean) (SweepResult :type "HitResult Structure (by ref)"))
  ;[0.7721 0.4346 1] Активация и раскраска отпечатков
  (if (== OtherComp (`self.DetectionSphere`))
    (`SceneComponent.SetVisibility` (`self.Decal_Fingerprint3`) true false)
    (`PrimitiveComponent.SetCollisionEnabled` (`self.collision3`) "QueryAndPhysics")))

(event `self.BoxOverlap4.OnComponentBeginOverlap`
  (params (OverlappedComponent :type "PrimitiveComponent Object Reference") (OtherActor :type "Actor Object Reference") (OtherComp :type "PrimitiveComponent Object Reference") (OtherBodyIndex :type Integer) (bFromSweep :type Boolean) (SweepResult :type "HitResult Structure (by ref)"))
  ;[0.7721 0.4346 1] Активация и раскраска отпечатков
  (if (== OtherComp (`self.DetectionSphere`))
    (`SceneComponent.SetVisibility` (`self.Decal_Fingerprint4_True`) true false)
    (`PrimitiveComponent.SetCollisionEnabled` (`self.collision4_t`) "QueryAndPhysics")))

(event `self.BoxOverlap5.OnComponentBeginOverlap`
  (params (OverlappedComponent :type "PrimitiveComponent Object Reference") (OtherActor :type "Actor Object Reference") (OtherComp :type "PrimitiveComponent Object Reference") (OtherBodyIndex :type Integer) (bFromSweep :type Boolean) (SweepResult :type "HitResult Structure (by ref)"))
  ;[0.7721 0.4346 1] Активация и раскраска отпечатков
  (if (== OtherComp (`self.DetectionSphere`))
    (`SceneComponent.SetVisibility` (`self.Decal_Fingerprint5`) true false)
    (`PrimitiveComponent.SetCollisionEnabled` (`self.collision5`) "QueryAndPhysics")))

(event `self.ReceiveBeginPlay`
  (bind (_x _y) (`KismetMathLibrary.BreakVector2D` (`WidgetLayoutLibrary.GetViewportSize`)))
  (bind _returnvalue (* (* (`KismetMathLibrary.Tan` (/ (`CameraComponent.FieldOfView` (`self.MinigameCamera`)) 2.0)) (`SpringArmComponent.TargetArmLength` (`self.SpringArm`))) 2.0))
  ;[1 0.7647 0.1854] Настройка освещения и фона
  (bind _outactors (`GameplayStatics.GetAllActorsOfClassWithTag` "/Script/Engine.DirectionalLight" "Day"))
  (`SceneComponent.SetVisibility` (`Light.LightComponent` (`|GetArrayItem` _outactors)) true false)
  (bind _outactors_2 (`GameplayStatics.GetAllActorsOfClassWithTag` "/Script/Engine.DirectionalLight" "Night"))
  (`SceneComponent.SetVisibility` (`Light.LightComponent` (`|GetArrayItem` _outactors_2)) false false)
  (`SceneComponent.SetWorldScale3D` (`self.Plane1`) (`KismetMathLibrary.MakeVector` (/ (* _returnvalue (/ _x _y)) 100.0) (/ _returnvalue 100.0) 1.0)))

(event `Key|E`
  (params (Key :type "Key Structure"))
  (bind (_worldlocation _worlddirection) (`PlayerController.DeprojectMousePositionToWorld` (`GameplayStatics.GetPlayerController` 0)))
  ;[0.1176 0.1462 0.2656] Поиск отпечатков
  (:`Pressed`
    (if (`self.bCheckPowder`)
      (set `self.bCheckPowder` false)
      (set `self.bAnimateActive` false)
      (bind _outactors (`GameplayStatics.GetAllActorsOfClass` "/Script/Engine.StaticMeshActor"))
      (bind (_outhit _returnvalue) (`KismetSystemLibrary.LineTraceSingleForObjects` _worldlocation (+ _worldlocation (* _worlddirection (`KismetMathLibrary.Conv_DoubleToVector` 2000.0))) (`|MakeArray` "ObjectTypeQuery1" :!type "EObjectTypeQuery Enum") false _outactors "None" false))
      (if _returnvalue
        (bind (_bblockinghit _binitialoverlap _time _distance _location _impactpoint) (`GameplayStatics.BreakHitResult` _outhit))
        (`SceneComponent.K2_SetWorldLocation` (`self.DetectionSphere`) _impactpoint false true)
        (`NiagaraFunctionLibrary.SpawnSystemAtLocation` "/Game/A_Surface_Footstep/Niagara_FX/ParticleSystems/PSN_Snow_Surface1.PSN_Snow_Surface1" _impactpoint)
        (`KismetSystemLibrary.Delay` 0.5)
        (`SceneComponent.K2_SetRelativeLocation` (`self.DetectionSphere`) (0.0 0.0 -20.0) false false)
        (`KismetSystemLibrary.Delay` 0.5)
        (set `self.bCheckPowder` true)
        (set `self.bAnimateActive` true)
        (else
          (set `self.bCheckPowder` true)
          (set `self.bAnimateActive` true))))))

(event `Start mini-game`
  (bind _returnvalue (`GameplayStatics.GetPlayerController` 0))
  (bind _fingerprintgameui (`self.FingerprintGameUI`))
  ;[0.3847 0.5209 1] Старт мини-игры
  (`self.EnableInput` _returnvalue)
  (bind _returnvalue_2 (`|CreateWidget` (`self.UI_FingerprintGame`)))
  (bind _output_get (set `self.FingerprintGameUI` _returnvalue_2))
  (`/Game/MiniGames/Mug_fingerprints/UI/UI_FingerprintGame.InitializeDossierItems` _output_get)
  (`UserWidget.AddToViewport` _output_get 0)
  (`PlayerController.SetViewTargetWithBlend` _returnvalue (`ActorComponent.GetOwner` (`self.MinigameCamera`)) 0.0 "VTBlend_Linear" 0.0 false)
  (set `PlayerController.bShowMouseCursor` true _returnvalue)
  (set `PlayerController.bEnableMouseOverEvents` true _returnvalue)
  (`WidgetBlueprintLibrary.SetInputMode_GameAndUIEx` _returnvalue _fingerprintgameui)
  (set `/Game/MiniGames/Mug_fingerprints/UI/UI_FingerprintGame.BP_Minigames` self _fingerprintgameui))

(event `End Mini-game`
  (params (IsSuccessful :type Boolean))
  (bind _returnvalue (`GameplayStatics.GetPlayerController` 0))
  (bind _returnvalue_2 (`GameplayStatics.GetPlayerController` 0))
  (bind _returnvalue_3 (`GameplayStatics.GetPlayerController` 0))
  (bind _returnvalue_4 (`GameplayStatics.GetGameInstance`))
  ;[1 0.3759 0.3261] Завершение мини игры
  (if IsSuccessful
    (`self.AddEvidence`))
  (`KismetSystemLibrary.Delay` 0.5 :!label _label)
  (`Widget.RemoveFromParent` (`self.FingerprintGameUI`))
  (bind _asbp_game_instance (cast `/Game/GameInstance/BP_GameInstance` _returnvalue_4))
  (message `/Game/GameInstance/BPI_LoadingScreen.ShowLoadingScreen` _returnvalue_4)
  (set `PlayerController.bShowMouseCursor` false _returnvalue_2)
  (set `PlayerController.bEnableMouseOverEvents` false _returnvalue_2)
  (`WidgetBlueprintLibrary.SetInputMode_GameOnly` _returnvalue_2)
  (bind _outactors (`GameplayStatics.GetAllActorsOfClassWithTag` "/Script/Engine.DirectionalLight" "Day"))
  (`SceneComponent.SetVisibility` (`Light.LightComponent` (`|GetArrayItem` _outactors)) false false)
  (bind _outactors_2 (`GameplayStatics.GetAllActorsOfClassWithTag` "/Script/Engine.DirectionalLight" "Night"))
  (`SceneComponent.SetVisibility` (`Light.LightComponent` (`|GetArrayItem` _outactors_2)) true false)
  (bind _current_camera (`/Game/GameInstance/BP_GameInstance.Current Camera` _asbp_game_instance))
  (if (`KismetSystemLibrary.IsValid` _current_camera)
    (`PlayerController.SetViewTargetWithBlend` _returnvalue_3 _current_camera 0.0 "VTBlend_Linear" 0.0 false)
    (else
      (`PlayerController.SetViewTargetWithBlend` _returnvalue_3 (`Controller.K2_GetPawn` _returnvalue_3) 0.0 "VTBlend_Linear" 0.0 false)))
  (`KismetSystemLibrary.Delay` 3.0)
  (`self.EnableInput` (`Controller.K2_GetPawn` _returnvalue) _returnvalue)
  (message `/Game/GameInstance/BPI_LoadingScreen.CloseLoadingScreen` _returnvalue_4)
  (`self.K2_DestroyActor`))

(event `/Game/MiniGames/BPI_GiveUp.GiveUp`
  ;[1 0.3759 0.3261] Завершение мини игры
  (goto _label))

(event `self.collision5.OnClicked`
  (params (TouchedComponent :type "PrimitiveComponent Object Reference") (ButtonPressed :type "Key Structure"))
  (bind _hoveredfingerprinttag (`self.HoveredFingerprintTag`))
  (bind _fingerprintgameui (`self.FingerprintGameUI`))
  ;[0.5657 1 0.9602] Выбор тега из взаимодействия с коллизией
  (`self.Hovered Tag` TouchedComponent)
  ;[0.3844 1 0.2667] Выбор отпечатка по его тегу
  (if (!= _hoveredfingerprinttag "None") :!label _label_2
    (set `self.SelectedFingerprint` (`BlueprintMapLibrary.Map_Find` (`self.FingerprintDictionary`) _hoveredfingerprinttag))
    (if (`KismetSystemLibrary.IsValid` _fingerprintgameui)
      (`/Game/MiniGames/Mug_fingerprints/UI/UI_FingerprintGame.UpdateSelectedFingerprint` _fingerprintgameui (`self.SelectedFingerprint`)))))

(event `self.collision2.OnClicked`
  (params (TouchedComponent :type "PrimitiveComponent Object Reference") (ButtonPressed :type "Key Structure"))
  ;[0.5657 1 0.9602] Выбор тега из взаимодействия с коллизией
  (`self.Hovered Tag` TouchedComponent)
  (goto _label_2))

(event `self.collision1.OnClicked`
  (params (TouchedComponent :type "PrimitiveComponent Object Reference") (ButtonPressed :type "Key Structure"))
  ;[0.5657 1 0.9602] Выбор тега из взаимодействия с коллизией
  (`self.Hovered Tag` TouchedComponent)
  (goto _label_2))

(event `InputAxis|RotateCup`
  (params (AxisValue :type "Float (single-precision)"))
  ;[1 0.7962 0.3395] Кручение кружки
  (if (`self.bIsDraggingCup`)
    (`SceneComponent.K2_AddRelativeRotation` (`self.mug`) (`KismetMathLibrary.MakeRotator` 0.0 0.0 (* AxisValue 3.0)) false false)))

(event `self.collision3.OnClicked`
  (params (TouchedComponent :type "PrimitiveComponent Object Reference") (ButtonPressed :type "Key Structure"))
  ;[0.5657 1 0.9602] Выбор тега из взаимодействия с коллизией
  (`self.Hovered Tag` TouchedComponent)
  (goto _label_2))

(event `self.collision4_t.OnClicked`
  (params (TouchedComponent :type "PrimitiveComponent Object Reference") (ButtonPressed :type "Key Structure"))
  ;[0.5657 1 0.9602] Выбор тега из взаимодействия с коллизией
  (`self.Hovered Tag` TouchedComponent)
  (goto _label_2))

(event `Key|RightMouseButton`
  (params (Key :type "Key Structure"))
  ;[1 0.7962 0.3395] Кручение кружки
  (:`Pressed`
    (if (`self.bAnimateActive`)
      (set `self.bIsDraggingCup` true)))
  (:`Released`
    (set `self.bIsDraggingCup` false)))

(fn `AddEvidence`
  (bind _asbp_game_instance (cast `/Game/GameInstance/BP_GameInstance` (`GameplayStatics.GetGameInstance`)))
  (`KismetArrayLibrary.Array_Add` (`/Game/GameInstance/BP_GameInstance.Dopros_evidence` _asbp_game_instance) (make `/Game/dopros/Round_info` (`KismetMathLibrary.Conv_IntToInt64` (`/Game/GameInstance/BP_GameInstance.ID+` _asbp_game_instance)) "NewEnumerator0" "NewEnumerator1" "Відбитки Лукаса Ламберта" null))
  (set `/Game/GameInstance/BP_GameInstance.ID+` (+ (`/Game/GameInstance/BP_GameInstance.ID+` _asbp_game_instance) 1) _asbp_game_instance))

(fn `Hovered Tag`
  (params (tag :type "ActorComponent Object Reference"))
  (set `self.HoveredFingerprintTag` (`|GetArrayItem` (`ActorComponent.ComponentTags` tag))))

(fn `UserConstructionScript`)