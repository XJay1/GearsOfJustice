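; Interactable letter actor that serves as the world entry point to the letter puzzle minigame.
; Overlapping LetterBox enables input and, if the letter is interactable, sets the in-range flag and shows a text prompt; leaving clears both.
; Pressing E in range spawns BP_LetterPuzzle at a hard-coded location, starts it, and hides the prompt and eight letter pieces.
; A separate LetterView event makes the Letter component visible.
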(event `LetterView`
  (`SceneComponent.SetVisibility` (`self.Letter`) true false))

(event `self.LetterBox.OnComponentBeginOverlap`
  (params (OverlappedComponent :type "PrimitiveComponent Object Reference") (OtherActor :type "Actor Object Reference") (OtherComp :type "PrimitiveComponent Object Reference") (OtherBodyIndex :type Integer) (bFromSweep :type Boolean) (SweepResult :type "HitResult Structure (by ref)"))
  ;[0.4417 0.4498 1] Надпись
  (`InputDeviceLibrary.GetPlayerControllerFromInputDevice` (struct))
  (`self.EnableInput` (`GameplayStatics.GetPlayerController` 0))
  (if (`self.bIsInteractableLetter`)
    (bind _output_get (set `self.bIsPlayerInRange` true))
    (`SceneComponent.SetVisibility` (`self.TextRender`) _output_get false)))

(event `self.ReceiveBeginPlay`)

(event `self.LetterBox.OnComponentEndOverlap`
  (params (OverlappedComponent :type "PrimitiveComponent Object Reference") (OtherActor :type "Actor Object Reference") (OtherComp :type "PrimitiveComponent Object Reference") (OtherBodyIndex :type Integer))
  ;[0.4417 0.4498 1] Надпись
  (`InputDeviceLibrary.GetPlayerControllerFromInputDevice` (struct))
  (bind _output_get (set `self.bIsPlayerInRange` false))
  (`SceneComponent.SetVisibility` (`self.TextRender`) _output_get false))

(event `Key|E`
  (params (Key :type "Key Structure"))
  ;[0.6615 0.6615 0.6615] Взаимодействие для начала мини игры
  (:`Pressed`
    (if (`self.bIsPlayerInRange`)
      (bind _returnvalue (`|SpawnActorFromClass` "/Game/MiniGames/Letter_puzzle/Blueprints/BP_LetterPuzzle.BP_LetterPuzzle_C" (`KismetMathLibrary.MakeTransform` (650.475888 230.758279 102.0)) "Undefined" "MultiplyWithRoot" null null))
      (`/Game/MiniGames/Letter_puzzle/Blueprints/BP_LetterPuzzle.Start mini-game` _returnvalue)
      (`SceneComponent.SetVisibility` (`self.TextRender`) false false)
      (`SceneComponent.SetVisibility` (`self.LetterPiece_08`) false false)
      (`SceneComponent.SetVisibility` (`self.LetterPiece_07`) false false)
      (`SceneComponent.SetVisibility` (`self.LetterPiece_06`) false false)
      (`SceneComponent.SetVisibility` (`self.LetterPiece_05`) false false)
      (`SceneComponent.SetVisibility` (`self.LetterPiece_04`) false false)
      (`SceneComponent.SetVisibility` (`self.LetterPiece_03`) false false)
      (`SceneComponent.SetVisibility` (`self.LetterPiece_02`) false false)
      (`SceneComponent.SetVisibility` (`self.LetterPiece_01`) false false))))

(fn `UserConstructionScript`)