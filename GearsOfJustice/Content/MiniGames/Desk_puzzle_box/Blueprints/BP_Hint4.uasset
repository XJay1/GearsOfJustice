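; BP_Hint4 is a hint note in the desk puzzle box minigame that the player can rotate to inspect.
; On BeginPlay it enables input and switches the player's view to its own camera.
; Holding the right mouse button sets a drag flag, letting the two RotateTable input axes apply world rotation to PlaneHints, scaled by RotationSpeed.
; The horizontal axis drives pitch and the vertical axis drives roll.
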(event `InputAxis|RotateTableHorizontal`
  (params (AxisValue :type "Float (single-precision)"))
  (bind _rotation_speed (`self.Rotation Speed`))
  ;[1 1 1] Поворот записки
  (set `self.Axis Horizontal` AxisValue)
  (if (`self.bIsHintDragging`) :!label _label
    (`SceneComponent.K2_AddWorldRotation` (`self.PlaneHints`) (`KismetMathLibrary.MakeRotator` (* (`self.Axis Vertical`) _rotation_speed) (* (`self.Axis Horizontal`) _rotation_speed)) false false)))

(event `InputAxis|RotateTableVertical`
  (params (AxisValue :type "Float (single-precision)"))
  ;[1 1 1] Поворот записки
  (set `self.Axis Vertical` AxisValue)
  (goto _label))

(event `Key|RightMouseButton`
  (params (Key :type "Key Structure"))
  ;[1 1 1] Поворот записки
  (:`Pressed`
    (set `self.bIsHintDragging` true))
  (:`Released`
    (set `self.bIsHintDragging` false)))

(event `self.ReceiveBeginPlay`
  (bind _returnvalue (`GameplayStatics.GetPlayerController` 0))
  (`self.EnableInput` _returnvalue)
  (`PlayerController.SetViewTargetWithBlend` _returnvalue (`ActorComponent.GetOwner` (`self.Camera`)) 0.0 "VTBlend_Linear" 0.0 false))

(fn `UserConstructionScript`)