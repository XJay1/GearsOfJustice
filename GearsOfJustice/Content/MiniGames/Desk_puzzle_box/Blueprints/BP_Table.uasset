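; BP_Table is an interactable table that launches the secret-table desk puzzle minigame.
; Overlapping its box enables player input and, if the table is interactable, shows an interact prompt widget, which hides when the overlap ends.
; Pressing E in range shows the GameInstance loading screen, spawns BP_SecretTable high above the world origin and starts its minigame, then closes the loading screen after a fixed delay.
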(event `self.TableBox.OnComponentBeginOverlap`
  (params (OverlappedComponent :type "PrimitiveComponent Object Reference") (OtherActor :type "Actor Object Reference") (OtherComp :type "PrimitiveComponent Object Reference") (OtherBodyIndex :type Integer) (bFromSweep :type Boolean) (SweepResult :type "HitResult Structure (by ref)"))
  (bind _widget (`self.Widget`))
  ;[0.4417 0.4498 1] Надпись
  (`InputDeviceLibrary.GetPlayerControllerFromInputDevice` (struct))
  (`self.EnableInput` (`GameplayStatics.GetPlayerController` 0))
  (if (`self.bIsInteractableTable`)
    (bind _output_get (set `self.bIsPlayerInRange` true))
    (`WidgetComponent.SetWidget` _widget (`self.W_Interact`))
    (`SceneComponent.SetVisibility` _widget _output_get false)
    (else
      (set `self.bIsPlayerInRange` false))))

(event `self.TableBox.OnComponentEndOverlap`
  (params (OverlappedComponent :type "PrimitiveComponent Object Reference") (OtherActor :type "Actor Object Reference") (OtherComp :type "PrimitiveComponent Object Reference") (OtherBodyIndex :type Integer))
  ;[0.4417 0.4498 1] Надпись
  (`InputDeviceLibrary.GetPlayerControllerFromInputDevice` (struct))
  (bind _output_get (set `self.bIsPlayerInRange` false))
  (`SceneComponent.SetVisibility` (`self.Widget`) _output_get false))

(event `Key|E` :consume false
  (params (Key :type "Key Structure"))
  ;[0.6615 0.6615 0.6615] Взаимодействие для начала мини игры
  (:`Pressed`
    (if (`self.bIsPlayerInRange`)
      (bind _asbp_game_instance (cast `/Game/GameInstance/BP_GameInstance` (`GameplayStatics.GetGameInstance`)))
      (`/Game/GameInstance/BP_GameInstance.ShowLoadingScreen` _asbp_game_instance)
      (bind _returnvalue (`|SpawnActorFromClass` "/Game/MiniGames/Desk_puzzle_box/Blueprints/BP_SecretTable.BP_SecretTable_C" (`KismetMathLibrary.MakeTransform` (0.0 0.0 10000.0)) "Undefined" "MultiplyWithRoot" null null))
      (`/Game/MiniGames/Desk_puzzle_box/Blueprints/BP_SecretTable.Start mini-game` _returnvalue)
      (`SceneComponent.SetVisibility` (`self.Widget`) false false)
      (`KismetSystemLibrary.Delay` 3.0)
      (`/Game/GameInstance/BP_GameInstance.CloseLoadingScreen` _asbp_game_instance))))

(fn `UserConstructionScript`)