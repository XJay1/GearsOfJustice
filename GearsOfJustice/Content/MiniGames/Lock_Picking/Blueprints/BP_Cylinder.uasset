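; Lockpicking minigame actor for a five-pin cylinder, one part of the locked locker minigame.
; Timelines animate a sliding pick; left click tests its position against pin hit zones.
; Hits set pins by a random roll whose chance rises after failures and resets on success; misses drop all pins.
; Five set pins, or the L key shortcut, turn the cylinder, notify BPLockedLocker, return its camera and destroy the actor.
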(event `self.ReceiveBeginPlay`
  (bind _returnvalue (`GameplayStatics.GetPlayerController` 0))
  (bind _ui_lockedlocker (`self.UI_LockedLocker`))
  ;[1 0.8498 0.385] Запуск части мини игры со взломом замка
  (`self.EnableInput` _returnvalue)
  (`PlayerController.SetViewTargetWithBlend` _returnvalue (`ActorComponent.GetOwner` (`self.Camera`)) 0.0 "VTBlend_Linear" 0.0 false)
  (`KismetSystemLibrary.Delay` 1.1)
  (`/Game/MiniGames/Lock_Picking/UI/UI_LockedLocker.Show text` _ui_lockedlocker)
  (set `/Game/MiniGames/Lock_Picking/UI/UI_LockedLocker.BP_Minigames` self _ui_lockedlocker))

(event `CheckCompletion`
  (bind _bp_lockedlocker (`self.BP_LockedLocker`))
  ;[1 0.2464 0.3563] Проверка на все задвинутые колышки
  (if (and (`self.PinActive1`) (`self.PinActive2`) (`self.PinActive3`) (`self.PinActive4`) (`self.PinActive5`))
    (set `self.bUnlockCylinder` true :!label _label)
    (set `self.bPinCheck` true)
    (`self.StopLockpickMoving`)
    (`GameplayStatics.PlaySound2D` "/Game/MiniGames/Lock_Picking/Sounds/Unlock.Unlock" 1.0 1.0 0.0 null null)
    (bind (_direction _alpha) (`Timeline|UnlockCylinder` :!via `PlayFromStart`)
      (:`Update`
        (`SceneComponent.K2_SetRelativeRotation` (`self.Cylinder_Brass-material`) (`KismetMathLibrary.MakeRotator` 0.0 (`KismetMathLibrary.Lerp` 0.0 180.0 _alpha)) false false))
      (:`Finished`
        (set `/Game/MiniGames/Lock_Picking/Blueprints/BP_LockedLocker.bCompleteLock1` true _bp_lockedlocker)
        (`/Game/MiniGames/Lock_Picking/Blueprints/BP_LockedLocker.OffOutline1` _bp_lockedlocker)
        (`/Game/MiniGames/Lock_Picking/UI/UI_LockedLocker.Fade` (`self.UI_LockedLocker`))
        (`KismetSystemLibrary.Delay` 1.0)
        (`PlayerController.SetViewTargetWithBlend` (`GameplayStatics.GetPlayerController` 0) (`ActorComponent.GetOwner` (`/Game/MiniGames/Lock_Picking/Blueprints/BP_LockedLocker.MinigameCamera` (`self.BP_LockedLocker`))) 0.0 "VTBlend_Linear" 0.0 false :!label _label_2)
        (set `/Game/MiniGames/Lock_Picking/UI/UI_LockedLocker.BP_Minigames` (`self.BP_LockedLocker`) (`self.UI_LockedLocker`))
        (`self.K2_DestroyActor`)))))

(event `/Game/MiniGames/BPI_GiveUp.GiveUp`
  ;[1 0.2464 0.3563] Проверка на все задвинутые колышки
  (`/Game/MiniGames/Lock_Picking/Blueprints/BP_LockedLocker.GiveUpPartCylinder` (`self.BP_LockedLocker`))
  (goto _label_2))

(event `Key|L`
  (params (Key :type "Key Structure"))
  ;[1 0.2464 0.3563] Проверка на все задвинутые колышки
  (:`Pressed`
    (goto _label)))

(event `PlayLockpickMoving`
  (bind _lockpick1 (`self.Lockpick1`))
  ;[0.8102 1 0.2686] Анимация движения отмычки
  (bind (_direction _alpha) (`Timeline|LockpickMoving` :!label _label_3)
    (:`Update`
      (`SceneComponent.K2_SetRelativeLocation` _lockpick1 (`KismetMathLibrary.MakeVector` (.x (`SceneComponent.RelativeLocation` _lockpick1)) (`KismetMathLibrary.Lerp` -14.0 -7.0 _alpha) (.z (`SceneComponent.RelativeLocation` _lockpick1))) false false))))

(event `LockpickMove`
  ;[0.8102 1 0.2686] Анимация движения отмычки
  (goto _label_3 :!via `PlayFromStart`))

(event `Key|E`
  (params (Key :type "Key Structure"))
  (bind _lockpick0 (`self.Lockpick0`))
  (bind _lockpick1 (`self.Lockpick1`))
  ;[0.3701 1 0.3964] Начать взлом замка
  (:`Pressed`
    (if (`self.StartMinigame`)
      (`/Game/MiniGames/Lock_Picking/UI/UI_LockedLocker.Hide text` (`self.UI_LockedLocker`))
      (set `self.StartMinigame` false)
      (bind (_direction _alpha) (`Timeline|StartLockpick0` :!via `PlayFromStart`)
        (:`Update`
          (`SceneComponent.K2_SetRelativeLocation` _lockpick0 (`KismetMathLibrary.MakeVector` (.x (`SceneComponent.RelativeLocation` _lockpick0)) (`KismetMathLibrary.Lerp` -15.0 -9.4 _alpha) (.z (`SceneComponent.RelativeLocation` _lockpick0))) false false))
        (:`Finished`
          (bind (_direction_2 _alpha_2) (`Timeline|StartLockpick1` :!via `PlayFromStart`)
            (:`Update`
              (`SceneComponent.K2_SetRelativeLocation` _lockpick1 (`KismetMathLibrary.MakeVector` (.x (`SceneComponent.RelativeLocation` _lockpick1)) (`KismetMathLibrary.Lerp` -19.0 -14.0 _alpha_2) (.z (`SceneComponent.RelativeLocation` _lockpick1))) false false))
            (:`Finished`
              (`self.LockpickMove`))))))))

(event `StopLockpickMoving`
  ;[0.8102 1 0.2686] Анимация движения отмычки
  (goto _label_3 :!via `Stop`))

(event `LockpickHitAnim`
  (bind _lockpick1 (`self.Lockpick1`))
  ;[1 0.9089 0.1698] Анимация удара отмычки
  (bind (_direction _alpha) (`Timeline|LockpickHit` :!via `PlayFromStart`)
    (:`Update`
      (`SceneComponent.K2_SetRelativeRotation` _lockpick1 (`KismetMathLibrary.MakeRotator` (.roll (`SceneComponent.RelativeRotation` _lockpick1)) (`KismetMathLibrary.Lerp` 0.0 -6.0 _alpha) (.yaw (`SceneComponent.RelativeRotation` _lockpick1))) false false))))

(event `Key|LeftMouseButton`
  (params (Key :type "Key Structure"))
  (bind _y (.y (`SceneComponent.RelativeLocation` (`self.Lockpick1`))))
  ;[0.4652 0.03996 1] Логика работы ударов по колышкам
  (:`Pressed`
    (if (`self.StartMinigame`)
      _
      (elif (not (`self.bPinCheck`))
        (`self.StopLockpickMoving`)
        (set `self.bPinCheck` true)
        (set `self.SelectedPin` null)
        (set `self.bAnyPinMatched` false)
        (for _array_element (`self.PinHitZones`)
          (bind (_pinreference _miny _maxy) (break `/Game/MiniGames/Lock_Picking/Blueprints/PinHitZoneStructure` _array_element))
          (if (and (> _y _miny) (< _y _maxy))
            (set `self.bAnyPinMatched` true)
            (bind _output_get (set `self.SelectedPinInt` _pinreference))
            (switch `int` _output_get
              (:`1`
                (set `self.SelectedPin` (`self.Pin1`))
                (set `self.SelectedLockPin` (`self.LockPin1`))
                (set `self.SelectedSpring` (`self.Spring_obj1`)))
              (:`2`
                (set `self.SelectedPin` (`self.Pin2`))
                (set `self.SelectedLockPin` (`self.LockPin2`))
                (set `self.SelectedSpring` (`self.Spring_obj2`)))
              (:`3`
                (set `self.SelectedPin` (`self.Pin3`))
                (set `self.SelectedLockPin` (`self.LockPin3`))
                (set `self.SelectedSpring` (`self.Spring_obj3`)))
              (:`4`
                (set `self.SelectedPin` (`self.Pin4`))
                (set `self.SelectedLockPin` (`self.LockPin4`))
                (set `self.SelectedSpring` (`self.Spring_obj4`)))
              (:`5`
                (set `self.SelectedPin` (`self.Pin5`))
                (set `self.SelectedLockPin` (`self.LockPin5`))
                (set `self.SelectedSpring` (`self.Spring_obj5`))))
            (if (<= (`KismetMathLibrary.RandomIntegerInRange` 0 100) (`self.Chance`))
              (set `self.Chance` 60)
              (switch `int` (`self.SelectedPinInt`)
                (:`1`
                  (set `self.PinActive1` true))
                (:`2`
                  (set `self.PinActive2` true))
                (:`3`
                  (set `self.PinActive3` true))
                (:`4`
                  (set `self.PinActive4` true))
                (:`5`
                  (set `self.PinActive5` true)))
              (`self.LockpickHitAnim`)
              (`GameplayStatics.PlaySound2D` "/Game/MiniGames/Lock_Picking/Sounds/PinUp.PinUp" 1.0 1.0 0.0 null null)
              (bind (_direction _alpha) (`Timeline|Fixation` :!via `PlayFromStart`)
                (:`Update`
                  (`SceneComponent.K2_SetRelativeLocation` (`self.SelectedPin`) (`KismetMathLibrary.MakeVector` 0.0 0.0 (`KismetMathLibrary.Lerp` 0.0 0.776124 _alpha)) false false)
                  (`SceneComponent.K2_SetRelativeLocation` (`self.SelectedLockPin`) (`KismetMathLibrary.MakeVector` 0.0 0.0 (`KismetMathLibrary.Lerp` 0.0 0.776124 _alpha)) false false)
                  (`SceneComponent.SetRelativeScale3D` (`self.SelectedSpring`) (`KismetMathLibrary.MakeVector` 1.0 1.0 (`KismetMathLibrary.Lerp` 1.0 0.67 _alpha))))
                (:`Finished`
                  (`self.CheckCompletion`)))
              (else
                (`self.LockpickHitAnim`)
                (`GameplayStatics.PlaySound2D` "/Game/MiniGames/Lock_Picking/Sounds/PinUp.PinUp" 1.0 1.0 0.0 null null)
                (bind (_direction_2 _alpha_2) (`Timeline|NotFixation` :!via `PlayFromStart`)
                  (:`Update`
                    (`SceneComponent.K2_SetRelativeLocation` (`self.SelectedPin`) (`KismetMathLibrary.MakeVector` 0.0 0.0 (`KismetMathLibrary.Lerp` 0.0 0.776124 _alpha_2)) false false)
                    (`SceneComponent.K2_SetRelativeLocation` (`self.SelectedLockPin`) (`KismetMathLibrary.MakeVector` 0.0 0.0 (`KismetMathLibrary.Lerp` 0.0 0.776124 _alpha_2)) false false)
                    (`SceneComponent.SetRelativeScale3D` (`self.SelectedSpring`) (`KismetMathLibrary.MakeVector` 1.0 1.0 (`KismetMathLibrary.Lerp` 1.0 0.67 _alpha_2))))
                  (:`Finished`
                    (set `self.Chance` (+ (`self.Chance`) 20))))))
            (else
              (`self.LockpickHitAnim`))))
        (if (`self.bAnyPinMatched`)
          (`KismetSystemLibrary.Delay` 0.5)
          (if (not (`self.bUnlockCylinder`))
            (`self.PlayLockpickMoving`)
            (set `self.bPinCheck` false))
          (else
            (`GameplayStatics.PlaySound2D` "/Game/MiniGames/Lock_Picking/Sounds/ResetPins.ResetPins" 1.0 1.0 0.0 null null)
            (bind (_direction_3 _alpha_3) (`Timeline|ResetAllPins` :!via `PlayFromStart`)
              (:`Update`
                (`SceneComponent.K2_SetRelativeLocation` (`self.Pin1`) (`KismetMathLibrary.MakeVector` 0.0 0.0 (`KismetMathLibrary.Lerp` 0.776124 0.0 _alpha_3)) false false)
                (`SceneComponent.K2_SetRelativeLocation` (`self.Pin2`) (`KismetMathLibrary.MakeVector` 0.0 0.0 (`KismetMathLibrary.Lerp` 0.776124 0.0 _alpha_3)) false false)
                (`SceneComponent.K2_SetRelativeLocation` (`self.Pin3`) (`KismetMathLibrary.MakeVector` 0.0 0.0 (`KismetMathLibrary.Lerp` 0.776124 0.0 _alpha_3)) false false)
                (`SceneComponent.K2_SetRelativeLocation` (`self.Pin4`) (`KismetMathLibrary.MakeVector` 0.0 0.0 (`KismetMathLibrary.Lerp` 0.776124 0.0 _alpha_3)) false false)
                (`SceneComponent.K2_SetRelativeLocation` (`self.Pin5`) (`KismetMathLibrary.MakeVector` 0.0 0.0 (`KismetMathLibrary.Lerp` 0.776124 0.0 _alpha_3)) false false)
                (`SceneComponent.K2_SetRelativeLocation` (`self.LockPin1`) (`KismetMathLibrary.MakeVector` 0.0 0.0 (`KismetMathLibrary.Lerp` 0.776124 0.0 _alpha_3)) false false)
                (`SceneComponent.K2_SetRelativeLocation` (`self.LockPin2`) (`KismetMathLibrary.MakeVector` 0.0 0.0 (`KismetMathLibrary.Lerp` 0.776124 0.0 _alpha_3)) false false)
                (`SceneComponent.K2_SetRelativeLocation` (`self.LockPin3`) (`KismetMathLibrary.MakeVector` 0.0 0.0 (`KismetMathLibrary.Lerp` 0.776124 0.0 _alpha_3)) false false)
                (`SceneComponent.K2_SetRelativeLocation` (`self.LockPin4`) (`KismetMathLibrary.MakeVector` 0.0 0.0 (`KismetMathLibrary.Lerp` 0.776124 0.0 _alpha_3)) false false)
                (`SceneComponent.K2_SetRelativeLocation` (`self.LockPin5`) (`KismetMathLibrary.MakeVector` 0.0 0.0 (`KismetMathLibrary.Lerp` 0.776124 0.0 _alpha_3)) false false)
                (`SceneComponent.SetRelativeScale3D` (`self.Spring_obj1`) (`KismetMathLibrary.MakeVector` 1.0 1.0 (`KismetMathLibrary.Lerp` 0.67 1.0 _alpha_3)))
                (`SceneComponent.SetRelativeScale3D` (`self.Spring_obj2`) (`KismetMathLibrary.MakeVector` 1.0 1.0 (`KismetMathLibrary.Lerp` 0.67 1.0 _alpha_3)))
                (`SceneComponent.SetRelativeScale3D` (`self.Spring_obj3`) (`KismetMathLibrary.MakeVector` 1.0 1.0 (`KismetMathLibrary.Lerp` 0.67 1.0 _alpha_3)))
                (`SceneComponent.SetRelativeScale3D` (`self.Spring_obj4`) (`KismetMathLibrary.MakeVector` 1.0 1.0 (`KismetMathLibrary.Lerp` 0.67 1.0 _alpha_3)))
                (`SceneComponent.SetRelativeScale3D` (`self.Spring_obj5`) (`KismetMathLibrary.MakeVector` 1.0 1.0 (`KismetMathLibrary.Lerp` 0.67 1.0 _alpha_3))))
              (:`Finished`
                (set `self.PinActive1` false)
                (set `self.PinActive2` false)
                (set `self.PinActive3` false)
                (set `self.PinActive4` false)
                (set `self.PinActive5` false)
                (`KismetSystemLibrary.Delay` 0.3)
                (`self.PlayLockpickMoving`)
                (set `self.bPinCheck` false)))))))))

(fn `UserConstructionScript`)