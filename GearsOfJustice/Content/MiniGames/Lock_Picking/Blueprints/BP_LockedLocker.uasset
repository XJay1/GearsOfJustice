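; Lock-picking minigame actor for a locked locker whose door opens once both cylinder locks are solved.
; The upper lock spawns BP_Cylinder; the lower lock uses a five-section rotatable key checked against a random code generated on BeginPlay, with matching pins outlined through custom depth.
; Timelines drive camera zooms, key and door animations, with right-mouse panning near the lower lock.
; Clicking the final collision ends the game with a placeholder evidence save.
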(event `Key|P`
  (params (Key :type "Key Structure"))
  (:`Pressed`
    (bind _returnvalue (`KismetMaterialLibrary.CreateDynamicMaterialInstance` "/Game/MiniGames/MI_Outline_InstForMinigame.MI_Outline_InstForMinigame"))
    (bind _output_get (set `self.DynamicMat` _returnvalue))
    (`MaterialInstanceDynamic.SetScalarParameterValue` _output_get "GlowIntensity" 0.0)
    (`MaterialInstanceDynamic.SetVectorParameterValue` _output_get "HighlightColor" (struct :`R` 1.0 :`G` 0.172445 :`A` 1.0))))

(event `OffOutline1`
  (`PrimitiveComponent.SetRenderCustomDepth` (`self.LockerMG_Cylinder1`) false))

(event `Start mini-game`
  (bind _returnvalue (`GameplayStatics.GetPlayerController` 0))
  ;[1 1 1] Запуск мини-игры
  (`self.EnableInput` _returnvalue)
  (bind _returnvalue_2 (`|CreateWidget` (`self.UI LockedLocker`)))
  (bind _output_get (set `self.LockedLockerUI` _returnvalue_2))
  (`UserWidget.AddToViewport` _output_get 0)
  (`PlayerController.SetViewTargetWithBlend` _returnvalue (`ActorComponent.GetOwner` (`self.MinigameCamera`)) 0.0 "VTBlend_Linear" 0.0 false)
  (set `PlayerController.bShowMouseCursor` true _returnvalue)
  (set `PlayerController.bEnableMouseOverEvents` true _returnvalue)
  (`WidgetBlueprintLibrary.SetInputMode_GameAndUIEx` _returnvalue (`self.LockedLockerUI`) "DoNotLock" false)
  (bind _outactors (`GameplayStatics.GetAllActorsOfClass` "/Game/MiniGames/Lock_Picking/Blueprints/BP_Locker.BP_Locker_C"))
  (bind _output (`|GetArrayItem` _outactors))
  (set `/Game/MiniGames/Lock_Picking/Blueprints/BP_Locker.bIsInteractableLocker` false _output)
  (set `/Game/MiniGames/Lock_Picking/Blueprints/BP_Locker.bIsPlayerInRange` false _output)
  (`PrimitiveComponent.SetRenderCustomDepth` (`self.LockerMG_Cylinder1`) true)
  (`PrimitiveComponent.SetRenderCustomDepth` (`self.CylinderCustom`) true))

(event `InputAxis|RotateTableHorizontal`
  (params (AxisValue :type "Float (single-precision)"))
  (bind _x (.x (`SceneComponent.K2_GetComponentLocation` (`self.CameraCylinder3`))))
  (bind _z (.z (`SceneComponent.K2_GetComponentLocation` (`self.CameraCylinder3`))))
  ;[1 0.8157 0.3331] Движение камерой вблизи к нижнему замку
  (if (`self.bIsRightMouseHeld`)
    (bind _output_get (set `self.CurrentOffset` (`KismetMathLibrary.MakeVector` (`KismetMathLibrary.FClamp` (+ AxisValue (.x (`self.CurrentOffset`))) (- _x 1.0) (+ _x 1.0)) (.y (`self.CurrentOffset`)) (`KismetMathLibrary.FClamp` (+ (stale `InputAxis|RotateTableVertical` AxisValue) (.z (`self.CurrentOffset`))) (- _z 1.0) (+ _z 1.0))) :!label _label))
    (`SceneComponent.K2_SetWorldLocation` (`self.MinigameCamera`) _output_get false false)))

(event `self.FinalCollision.OnClicked`
  (params (TouchedComponent :type "PrimitiveComponent Object Reference") (ButtonPressed :type "Key Structure"))
  (bind _returnvalue (`GameplayStatics.GetPlayerController` 0))
  ;[1 0.07441 0.02465] Завершение мини-игры
  (`/Game/MiniGames/Lock_Picking/UI/UI_LockedLocker.Final Stage` (`self.LockedLockerUI`))
  (`KismetSystemLibrary.Delay` 2.0)
  (`KismetSystemLibrary.PrintString` "Будет сохранение улики")
  (`KismetSystemLibrary.Delay` 2.0)
  (`Widget.RemoveFromParent` (`self.LockedLockerUI`))
  (set `PlayerController.bShowMouseCursor` false _returnvalue)
  (set `PlayerController.bEnableMouseOverEvents` false _returnvalue)
  (`WidgetBlueprintLibrary.SetInputMode_GameOnly` _returnvalue)
  (`self.K2_DestroyActor`))

(event `InputAxis|RotateTableVertical`
  (params (AxisValue :type "Float (single-precision)"))
  ;[1 0.8157 0.3331] Движение камерой вблизи к нижнему замку
  (if (`self.bIsRightMouseHeld`)
    (goto _label)))

(event `self.Cylinder1ColBox.OnClicked`
  (params (TouchedComponent :type "PrimitiveComponent Object Reference") (ButtonPressed :type "Key Structure"))
  (bind _minigamecamera (`self.MinigameCamera`))
  (bind _cameracylinder1 (`self.CameraCylinder1`))
  ;[0.1971 0.4718 1] Открытие взлома замка сверху
  (`PrimitiveComponent.SetCollisionEnabled` TouchedComponent "NoCollision")
  (set `self.Start Location` (`SceneComponent.K2_GetComponentLocation` _minigamecamera))
  (set `self.Start Rotation` (`SceneComponent.K2_GetComponentRotation` _minigamecamera))
  (set `self.Target Location` (`SceneComponent.K2_GetComponentLocation` _cameracylinder1))
  (set `self.Target Rotation` (`SceneComponent.K2_GetComponentRotation` _cameracylinder1))
  (`/Game/MiniGames/Lock_Picking/UI/UI_LockedLocker.Fade` (`self.LockedLockerUI`))
  (`self.ZoomIn`)
  (set `self.bIsZoom` false)
  (`KismetSystemLibrary.Delay` 1.0)
  (bind _returnvalue (`|SpawnActorFromClass` "/Game/MiniGames/Lock_Picking/Blueprints/BP_Cylinder.BP_Cylinder_C" (`KismetMathLibrary.MakeTransform` (0.0 0.0 -600.0)) "Undefined" "MultiplyWithRoot" null null))
  (set `/Game/MiniGames/Lock_Picking/Blueprints/BP_Cylinder.BP_LockedLocker` self _returnvalue)
  (set `/Game/MiniGames/Lock_Picking/Blueprints/BP_Cylinder.UI_LockedLocker` (`self.LockedLockerUI`) _returnvalue)
  (`SceneComponent.K2_SetWorldLocation` (`self.MinigameCamera`) (`self.Start Location`) false false)
  (`SceneComponent.K2_SetWorldRotation` (`self.MinigameCamera`) (`self.Start Rotation`) false false))

(event `Key|RightMouseButton`
  (params (Key :type "Key Structure"))
  (bind _bisnearzoomcylinder2 (`self.bIsNearZoomCylinder2`))
  ;[1 0.8157 0.3331] Движение камерой вблизи к нижнему замку
  (:`Pressed`
    (if _bisnearzoomcylinder2
      (set `self.bIsRightMouseHeld` true)))
  (:`Released`
    (if _bisnearzoomcylinder2
      (set `self.bIsRightMouseHeld` false)
      (bind _output_get (set `self.CurrentOffset` (`SceneComponent.K2_GetComponentLocation` (`self.CameraCylinder3`))))
      (`SceneComponent.K2_SetWorldLocation` (`self.MinigameCamera`) _output_get false false))))

(event `self.Cylinder2ColBox.OnClicked`
  (params (TouchedComponent :type "PrimitiveComponent Object Reference") (ButtonPressed :type "Key Structure"))
  (bind _key_keyhandle (`self.Key_KeyHandle`))
  (bind _minigamecamera (`self.MinigameCamera`))
  (bind _cameracylinder2 (`self.CameraCylinder2`))
  ;[0.03208 0.07919 1] Открытие взлома замка внизу
  (`PrimitiveComponent.SetCollisionEnabled` TouchedComponent "NoCollision")
  (`PrimitiveComponent.SetRenderCustomDepth` (`self.CylinderCustom`) false)
  (`SceneComponent.SetVisibility` (`self.PostProcess`) false false)
  (`SceneComponent.SetVisibility` (`self.PostProcessPins`) true false)
  (set `self.Start Location` (`SceneComponent.K2_GetComponentLocation` _minigamecamera))
  (set `self.Start Rotation` (`SceneComponent.K2_GetComponentRotation` _minigamecamera))
  (set `self.Target Location` (`SceneComponent.K2_GetComponentLocation` _cameracylinder2))
  (set `self.Target Rotation` (`SceneComponent.K2_GetComponentRotation` _cameracylinder2))
  (`self.ZoomIn`)
  (set `self.bIsZoom` false)
  (bind (_direction _alpha) (`Timeline|KeyMoveIn` :!via `PlayFromStart`)
    (:`Update`
      (`SceneComponent.K2_SetWorldLocation` _key_keyhandle (`KismetMathLibrary.MakeVector` (.x (`SceneComponent.K2_GetComponentLocation` _key_keyhandle)) (`KismetMathLibrary.Lerp` 150.0 58.0 _alpha) (.z (`SceneComponent.K2_GetComponentLocation` _key_keyhandle))) false false))
    (:`Finished`
      (`/Game/MiniGames/Lock_Picking/UI/UI_LockedLocker.ShowHint2` (`self.LockedLockerUI`)))))

(event `Key|K`
  (params (Key :type "Key Structure"))
  ;[0 0 0] Отладка
  (:`Pressed`
    (for _array_element (`self.KeyCode`)
      (`KismetSystemLibrary.PrintString` (`KismetStringLibrary.Conv_IntToString` _array_element)))))

(event `ZoomIn`
  ;[1 0.1445 0.9239] Приближение
  (set `self.bIsZoom` true)
  (bind (_direction _alpha) (`Timeline|Zoom` :!via `PlayFromStart`)
    (:`Update`
      (`SceneComponent.K2_SetWorldLocation` (`self.MinigameCamera`) (`KismetMathLibrary.VLerp` (`self.Start Location`) (`self.Target Location`) _alpha) false false)
      (`SceneComponent.K2_SetWorldRotation` (`self.MinigameCamera`) (`KismetMathLibrary.RLerp` (`self.Start Rotation`) (`self.Target Rotation`) _alpha) false false))))

(event `self.CollisionBoxDoor.OnClicked`
  (params (TouchedComponent :type "PrimitiveComponent Object Reference") (ButtonPressed :type "Key Structure"))
  ;[0.5466 1 0.08332] Проверка на возможность открытия двери
  (if (and (`self.bCompleteLock1`) (`self.bCompleteLock2`))
    (`GameplayStatics.PlaySound2D` "/Game/MiniGames/Lock_Picking/Sounds/DoorOpen.DoorOpen" 1.0 1.0 0.0 null null)
    (bind (_direction _alpha) (`Timeline|DoorOpen` :!via `PlayFromStart`)
      (:`Update`
        (`SceneComponent.K2_SetWorldRotation` (`self.Door`) (`KismetMathLibrary.MakeRotator` 0.0 0.0 (`KismetMathLibrary.Lerp` 0.0 90.0 _alpha)) false false)))
    (else
      (`GameplayStatics.PlaySound2D` "/Game/MiniGames/Lock_Picking/Sounds/ClosedDoor.ClosedDoor" 1.0 1.0 0.0 null null)
      (bind (_direction_2 _alpha_2) (`Timeline|DoorNotOpen` :!via `PlayFromStart`)
        (:`Update`
          (`SceneComponent.K2_SetWorldRotation` (`self.Door`) (`KismetMathLibrary.MakeRotator` 0.0 0.0 (`KismetMathLibrary.Lerp` 0.0 1.0 _alpha_2)) false false))))))

(event `ZoomOut`
  ;[0.2031 0.06082 0.1788] Отдаление
  (bind (_direction _alpha) (`Timeline|CameraBack` :!via `PlayFromStart` :!label _label_2)
    (:`Update`
      (`SceneComponent.K2_SetWorldLocation` (`self.MinigameCamera`) (`KismetMathLibrary.VLerp` (`self.Target Location`) (`self.Start Location`) _alpha) false false)
      (`SceneComponent.K2_SetWorldRotation` (`self.MinigameCamera`) (`KismetMathLibrary.RLerp` (`self.Target Rotation`) (`self.Start Rotation`) _alpha true) false false))
    (:`Finished`
      (set `self.bIsZoom` false)
      (`SceneComponent.SetVisibility` (`self.SpotLight`) false false)
      (set `self.bIsNearZoomCylinder2` false))))

(event `Key|Q`
  (params (Key :type "Key Structure"))
  ;[0.2031 0.06082 0.1788] Отдаление
  (:`Pressed`
    (if (`self.bIsZoom`)
      (`PrimitiveComponent.SetCollisionEnabled` (`self.SelectedCollision`) "QueryAndProbe")
      (goto _label_2 :!via `PlayFromStart`))))

(event `self.ReceiveBeginPlay`
  (bind _pinmatrix (`self.PinMatrix`))
  ;[0 0.8639 1] Генерация пароля для нижнего замка
  (for _ (range 5)
    (`KismetArrayLibrary.Array_Add` (`self.KeyCode`) (`KismetMathLibrary.RandomIntegerInRange` 0 3)))
  (`KismetArrayLibrary.Array_Add` _pinmatrix (make `/Game/MiniGames/Lock_Picking/Blueprints/PinsRowStructure` (`|MakeArray` (`self.LockerMG_PinOne_0`) (`self.LockerMG_PinOne_1`) (`self.LockerMG_PinOne_2`) (`self.LockerMG_PinOne_3`))))
  (`KismetArrayLibrary.Array_Add` _pinmatrix (make `/Game/MiniGames/Lock_Picking/Blueprints/PinsRowStructure` (`|MakeArray` (`self.LockerMG_PinTwo_0`) (`self.LockerMG_PinTwo_1`) (`self.LockerMG_PinTwo_2`) (`self.LockerMG_PinTwo_3`))))
  (`KismetArrayLibrary.Array_Add` _pinmatrix (make `/Game/MiniGames/Lock_Picking/Blueprints/PinsRowStructure` (`|MakeArray` (`self.LockerMG_PinThree_0`) (`self.LockerMG_PinThree_1`) (`self.LockerMG_PinThree_2`) (`self.LockerMG_PinThree_3`))))
  (`KismetArrayLibrary.Array_Add` _pinmatrix (make `/Game/MiniGames/Lock_Picking/Blueprints/PinsRowStructure` (`|MakeArray` (`self.LockerMG_PinFour_0`) (`self.LockerMG_PinFour_1`) (`self.LockerMG_PinFour_2`) (`self.LockerMG_PinFour_3`))))
  (`KismetArrayLibrary.Array_Add` _pinmatrix (make `/Game/MiniGames/Lock_Picking/Blueprints/PinsRowStructure` (`|MakeArray` (`self.LockerMG_PinFive_0`) (`self.LockerMG_PinFive_1`) (`self.LockerMG_PinFive_2`) (`self.LockerMG_PinFive_3`))))
  (for (_array_element _array_index) (`self.KeyCode`)
    (`PrimitiveComponent.SetRenderCustomDepth` (`|GetArrayItem` (`.PinsArray_4_BFC1055E4F20021CD976258D94FD17E7` (break `/Game/MiniGames/Lock_Picking/Blueprints/PinsRowStructure` (`|GetArrayItem` (`self.PinMatrix`) _array_index))) _array_element) true)))

(event `self.KeyCollision.OnClicked`
  (params (TouchedComponent :type "PrimitiveComponent Object Reference") (ButtonPressed :type "Key Structure"))
  (bind _minigamecamera (`self.MinigameCamera`))
  (bind _cameracylinder4 (`self.CameraCylinder4`))
  ;[0.3937 0.6265 1] Приближение к ключу
  (bind _output_get (set `self.SelectedCollision` TouchedComponent))
  (`PrimitiveComponent.SetCollisionEnabled` _output_get "NoCollision")
  (set `self.Start Location` (`SceneComponent.K2_GetComponentLocation` _minigamecamera))
  (set `self.Start Rotation` (`SceneComponent.K2_GetComponentRotation` _minigamecamera))
  (set `self.Target Location` (`SceneComponent.K2_GetComponentLocation` _cameracylinder4))
  (set `self.Target Rotation` (`SceneComponent.K2_GetComponentRotation` _cameracylinder4))
  (`self.ZoomIn`))

(event `self.NearCylinder2ColBox.OnClicked`
  (params (TouchedComponent :type "PrimitiveComponent Object Reference") (ButtonPressed :type "Key Structure"))
  (bind _minigamecamera (`self.MinigameCamera`))
  (bind _cameracylinder3 (`self.CameraCylinder3`))
  ;[1 1 1] Приближение к замку снизу
  (bind _output_get (set `self.SelectedCollision` TouchedComponent))
  (`PrimitiveComponent.SetCollisionEnabled` _output_get "NoCollision")
  (set `self.bIsNearZoomCylinder2` true)
  (set `self.Start Location` (`SceneComponent.K2_GetComponentLocation` _minigamecamera))
  (set `self.Start Rotation` (`SceneComponent.K2_GetComponentRotation` _minigamecamera))
  (set `self.Target Location` (`SceneComponent.K2_GetComponentLocation` _cameracylinder3))
  (set `self.Target Rotation` (`SceneComponent.K2_GetComponentRotation` _cameracylinder3))
  (`self.ZoomIn`)
  (`SceneComponent.SetVisibility` (`self.SpotLight`) true false)
  (set `self.CurrentOffset` (`SceneComponent.K2_GetComponentLocation` (`self.CameraCylinder3`))))

(event `self.CollisionSection1.OnClicked`
  (params (TouchedComponent :type "PrimitiveComponent Object Reference") (ButtonPressed :type "Key Structure"))
  ;[1 0.5534 0.1706] Прокручивание секций ключа
  (if (not (`self.bIsKeyRotating`))
    (set `self.bIsKeyRotating` true)
    (bind _output_get (set `self.StartRotationKey` (.roll (`SceneComponent.RelativeRotation` (`self.Key_Section1`)))))
    (set `self.TargetRotationKey` (- _output_get (`self.RotationStep`)))
    (bind _result (`/Engine/EditorBlueprintResources/StandardMacros.IncrementInt` (`self.Section1_Value`))
      (:`  `
        (bind _output_get_2 (set `self.Section1_Value` _result))
        (if (> _output_get_2 3)
          (set `self.Section1_Value` 0)
          (bind (_direction _alpha) (`Timeline|RotateKeySection1` :!via `PlayFromStart` :!label _label_3)
            (:`Update`
              (`SceneComponent.K2_SetRelativeRotation` (`self.Key_Section1`) (`KismetMathLibrary.MakeRotator` (`KismetMathLibrary.Lerp` (`self.StartRotationKey`) (`self.TargetRotationKey`) _alpha)) false false))
            (:`Finished`
              (set `self.bIsKeyRotating` false)))
          (else
            (goto _label_3 :!via `PlayFromStart`)))))))

(event `self.CollisionSection2.OnClicked`
  (params (TouchedComponent :type "PrimitiveComponent Object Reference") (ButtonPressed :type "Key Structure"))
  ;[1 0.5534 0.1706] Прокручивание секций ключа
  (if (not (`self.bIsKeyRotating`))
    (set `self.bIsKeyRotating` true)
    (bind _output_get (set `self.StartRotationKey` (.roll (`SceneComponent.RelativeRotation` (`self.Key_Section2`)))))
    (set `self.TargetRotationKey` (- _output_get (`self.RotationStep`)))
    (bind _result (`/Engine/EditorBlueprintResources/StandardMacros.IncrementInt` (`self.Section2_Value`))
      (:`  `
        (bind _output_get_2 (set `self.Section2_Value` _result))
        (if (> _output_get_2 3)
          (set `self.Section2_Value` 0)
          (bind (_direction _alpha) (`Timeline|RotateKeySection2` :!via `PlayFromStart` :!label _label_4)
            (:`Update`
              (`SceneComponent.K2_SetRelativeRotation` (`self.Key_Section2`) (`KismetMathLibrary.MakeRotator` (`KismetMathLibrary.Lerp` (`self.StartRotationKey`) (`self.TargetRotationKey`) _alpha)) false false))
            (:`Finished`
              (set `self.bIsKeyRotating` false)))
          (else
            (goto _label_4 :!via `PlayFromStart`)))))))

(event `self.KeyRingCollision.OnClicked`
  (params (TouchedComponent :type "PrimitiveComponent Object Reference") (ButtonPressed :type "Key Structure"))
  (bind _key_keyhandle (`self.Key_KeyHandle`))
  (bind _key_keyhandle_2 (`self.Key_KeyHandle`))
  (bind _minigamecamera (`self.MinigameCamera`))
  (bind _cameracylinder5 (`self.CameraCylinder5`))
  (bind _startpositioncamera (`self.StartPositionCamera`))
  (bind _cameracylinder5_2 (`self.CameraCylinder5`))
  (bind _keycode (`self.KeyCode`))
  ;[0.8084 0.5071 1] Проверка верности секций ключа и пароля
  (if (not (`self.bIsKeyRotating`))
    (set `self.bIsKeyRotating` true)
    (set `self.Start Location` (`SceneComponent.K2_GetComponentLocation` _minigamecamera))
    (set `self.Start Rotation` (`SceneComponent.K2_GetComponentRotation` _minigamecamera))
    (set `self.Target Location` (`SceneComponent.K2_GetComponentLocation` _cameracylinder5))
    (set `self.Target Rotation` (`SceneComponent.K2_GetComponentRotation` _cameracylinder5))
    (`self.ZoomIn`)
    (set `self.bIsZoom` false)
    (bind (_direction _alpha) (`Timeline|KeyZoomIn` :!via `PlayFromStart`)
      (:`Update`
        (`SceneComponent.K2_SetWorldLocation` _key_keyhandle_2 (`KismetMathLibrary.MakeVector` (.x (`SceneComponent.K2_GetComponentLocation` _key_keyhandle_2)) (`KismetMathLibrary.Lerp` 58.0 38.0 _alpha) (.z (`SceneComponent.K2_GetComponentLocation` _key_keyhandle_2))) false false))
      (:`Finished`
        (if (and (== (`self.Section1_Value`) (`|GetArrayItem` _keycode)) (== (`self.Section2_Value`) (`|GetArrayItem` _keycode 1)) (== (`self.Section3_Value`) (`|GetArrayItem` _keycode 2)) (== (`self.Section4_Value`) (`|GetArrayItem` _keycode 3)) (== (`self.Section5_Value`) (`|GetArrayItem` _keycode 4)))
          (`GameplayStatics.PlaySound2D` "/Game/MiniGames/Lock_Picking/Sounds/Unlock.Unlock" 1.0 1.0 0.0 null null :!label _label_5)
          (bind (_direction_2 _alpha_2) (`Timeline|OpenCylinder2` :!via `PlayFromStart`)
            (:`Update`
              (`SceneComponent.K2_SetWorldRotation` (`self.Key_KeyHandle`) (`KismetMathLibrary.MakeRotator` (`KismetMathLibrary.Lerp` 0.0 360.0 _alpha_2) 0.0 -90.0) false false)
              (`SceneComponent.K2_SetWorldRotation` (`self.CylinderCustom`) (`KismetMathLibrary.MakeRotator` (`KismetMathLibrary.Lerp` 0.0 360.0 _alpha_2) 0.0 -90.0) false false))
            (:`Finished`
              (set `self.bCompleteLock2` true)
              (set `self.Start Location` (`SceneComponent.K2_GetComponentLocation` _startpositioncamera))
              (set `self.Start Rotation` (`SceneComponent.K2_GetComponentRotation` _startpositioncamera))
              (set `self.Target Location` (`SceneComponent.K2_GetComponentLocation` _cameracylinder5_2))
              (set `self.Target Rotation` (`SceneComponent.K2_GetComponentRotation` _cameracylinder5_2))
              (`SceneComponent.SetVisibility` (`self.PostProcess`) true false)
              (`SceneComponent.SetVisibility` (`self.PostProcessPins`) false false)
              (`self.ZoomOut`)
              (`/Game/MiniGames/Lock_Picking/UI/UI_LockedLocker.HideHint2` (`self.LockedLockerUI`))
              (for (_array_element _array_index) (`self.KeyCode`)
                (`PrimitiveComponent.SetRenderCustomDepth` (`|GetArrayItem` (`.PinsArray_4_BFC1055E4F20021CD976258D94FD17E7` (break `/Game/MiniGames/Lock_Picking/Blueprints/PinsRowStructure` (`|GetArrayItem` (`self.PinMatrix`) _array_index))) _array_element) false))))
          (else
            (`GameplayStatics.PlaySound2D` "/Game/MiniGames/Lock_Picking/Sounds/ClosedCylinder.ClosedCylinder" 1.0 1.0 0.0 null null)
            (bind (_direction_3 _alpha_3) (`Timeline|NotOpen` :!via `PlayFromStart`)
              (:`Update`
                (`SceneComponent.K2_SetWorldRotation` (`self.Key_KeyHandle`) (`KismetMathLibrary.MakeRotator` (`KismetMathLibrary.Lerp` 0.0 10.0 _alpha_3) 0.0 -90.0) false false)
                (`SceneComponent.K2_SetWorldRotation` (`self.CylinderCustom`) (`KismetMathLibrary.MakeRotator` (`KismetMathLibrary.Lerp` 0.0 10.0 _alpha_3) 0.0 -90.0) false false))
              (:`Finished`
                (`self.ZoomOut`)
                (bind (_direction_4 _alpha_4) (`Timeline|KeyZoomOut` :!via `PlayFromStart`)
                  (:`Update`
                    (`SceneComponent.K2_SetWorldLocation` _key_keyhandle (`KismetMathLibrary.MakeVector` (.x (`SceneComponent.K2_GetComponentLocation` _key_keyhandle)) (`KismetMathLibrary.Lerp` 38.0 58.0 _alpha_4) (.z (`SceneComponent.K2_GetComponentLocation` _key_keyhandle))) false false))
                  (:`Finished`
                    (set `self.bIsKeyRotating` false)))))))))))

(event `self.CollisionSection3.OnClicked`
  (params (TouchedComponent :type "PrimitiveComponent Object Reference") (ButtonPressed :type "Key Structure"))
  ;[1 0.5534 0.1706] Прокручивание секций ключа
  (if (not (`self.bIsKeyRotating`))
    (set `self.bIsKeyRotating` true)
    (bind _output_get (set `self.StartRotationKey` (.roll (`SceneComponent.RelativeRotation` (`self.Key_Section3`)))))
    (set `self.TargetRotationKey` (- _output_get (`self.RotationStep`)))
    (bind _result (`/Engine/EditorBlueprintResources/StandardMacros.IncrementInt` (`self.Section3_Value`))
      (:`  `
        (bind _output_get_2 (set `self.Section3_Value` _result))
        (if (> _output_get_2 3)
          (set `self.Section3_Value` 0)
          (bind (_direction _alpha) (`Timeline|RotateKeySection3` :!via `PlayFromStart` :!label _label_6)
            (:`Update`
              (`SceneComponent.K2_SetRelativeRotation` (`self.Key_Section3`) (`KismetMathLibrary.MakeRotator` (`KismetMathLibrary.Lerp` (`self.StartRotationKey`) (`self.TargetRotationKey`) _alpha)) false false))
            (:`Finished`
              (set `self.bIsKeyRotating` false)))
          (else
            (goto _label_6 :!via `PlayFromStart`)))))))

(event `Key|L`
  (params (Key :type "Key Structure"))
  ;[0.8084 0.5071 1] Проверка верности секций ключа и пароля
  (:`Pressed`
    (goto _label_5)))

(event `self.CollisionSection4.OnClicked`
  (params (TouchedComponent :type "PrimitiveComponent Object Reference") (ButtonPressed :type "Key Structure"))
  ;[1 0.5534 0.1706] Прокручивание секций ключа
  (if (not (`self.bIsKeyRotating`))
    (set `self.bIsKeyRotating` true)
    (bind _output_get (set `self.StartRotationKey` (.roll (`SceneComponent.RelativeRotation` (`self.Key_Section4`)))))
    (set `self.TargetRotationKey` (- _output_get (`self.RotationStep`)))
    (bind _result (`/Engine/EditorBlueprintResources/StandardMacros.IncrementInt` (`self.Section4_Value`))
      (:`  `
        (bind _output_get_2 (set `self.Section4_Value` _result))
        (if (> _output_get_2 3)
          (set `self.Section4_Value` 0)
          (bind (_direction _alpha) (`Timeline|RotateKeySection4` :!via `PlayFromStart` :!label _label_7)
            (:`Update`
              (`SceneComponent.K2_SetRelativeRotation` (`self.Key_Section4`) (`KismetMathLibrary.MakeRotator` (`KismetMathLibrary.Lerp` (`self.StartRotationKey`) (`self.TargetRotationKey`) _alpha)) false false))
            (:`Finished`
              (set `self.bIsKeyRotating` false)))
          (else
            (goto _label_7 :!via `PlayFromStart`)))))))

(event `self.CollisionSection5.OnClicked`
  (params (TouchedComponent :type "PrimitiveComponent Object Reference") (ButtonPressed :type "Key Structure"))
  ;[1 0.5534 0.1706] Прокручивание секций ключа
  (if (not (`self.bIsKeyRotating`))
    (set `self.bIsKeyRotating` true)
    (bind _output_get (set `self.StartRotationKey` (.roll (`SceneComponent.RelativeRotation` (`self.Key_Section5`)))))
    (set `self.TargetRotationKey` (- _output_get (`self.RotationStep`)))
    (bind _result (`/Engine/EditorBlueprintResources/StandardMacros.IncrementInt` (`self.Section5_Value`))
      (:`  `
        (bind _output_get_2 (set `self.Section5_Value` _result))
        (if (> _output_get_2 3)
          (set `self.Section5_Value` 0)
          (bind (_direction _alpha) (`Timeline|RotateKeySection5` :!via `PlayFromStart` :!label _label_8)
            (:`Update`
              (`SceneComponent.K2_SetRelativeRotation` (`self.Key_Section5`) (`KismetMathLibrary.MakeRotator` (`KismetMathLibrary.Lerp` (`self.StartRotationKey`) (`self.TargetRotationKey`) _alpha)) false false))
            (:`Finished`
              (set `self.bIsKeyRotating` false)))
          (else
            (goto _label_8 :!via `PlayFromStart`)))))))

(fn `UserConstructionScript`)