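; BP_TemporaryDataHolderForPC is a prototype data container for the state of the in-game PC puzzle.
; It holds mail clue parts, found parts, a hack hint flag and hack decryption progress as separate variables.
; SetPCGameData unpacks a PCGameData struct into those variables, and GetPCGameData packs them back into the struct, with no other logic.
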(fn SetPCGameData
  (params (PCGameData :type STR%20Data%20for%20PC%20Structure))
  (Variables|Default|SetMailCluePart1 (.mailcluepart1 PCGameData))
  (Variables|Default|SetMailCluePart2 (.mailcluepart2 PCGameData))
  (Variables|Default|SetMailCluePart3 (.mailcluepart3 PCGameData))
  (Variables|Default|SetFoundParts (.foundparts PCGameData))
  (Variables|Default|SetHackHintIsFound (.hackhintisfound PCGameData))
  (Variables|Default|SetHackDecrypted1 (.hackdecrypted1 PCGameData))
  (Variables|Default|SetHackDecrypted2 (.hackdecrypted2 PCGameData))
  (Variables|Default|SetHackDecrypted3 (.hackdecrypted3 PCGameData))
  (return))

(fn GetPCGameData
  (return (Utilities|Struct|MakeSTR_DataForPC (Variables|Default|GetMailCluePart1) (Variables|Default|GetMailCluePart2) (Variables|Default|GetMailCluePart3) (Variables|Default|GetFoundParts) (Variables|Default|GetHackHintIsFound) (Variables|Default|GetHackDecrypted1) (Variables|Default|GetHackDecrypted2) (Variables|Default|GetHackDecrypted3))))