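; BP_Computer is an interactable computer that opens its home screen UI when E is pressed in range.
; Overlapping InteractionTrigger enables input for player 0, sets the range flag and shows the prompt widget, and leaving clears both flag and prompt.
; Pressing E while in range adds a new ComputerInterface widget to the viewport, switching to UI-only input with a visible cursor.
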(event `self.InteractionTrigger.OnComponentBeginOverlap`
  (params (OverlappedComponent :type "PrimitiveComponent Object Reference") (OtherActor :type "Actor Object Reference") (OtherComp :type "PrimitiveComponent Object Reference") (OtherBodyIndex :type Integer) (bFromSweep :type Boolean) (SweepResult :type "HitResult Structure (by ref)"))
  (bind _widget (`self.Widget`))
  (bind _w_interact (`self.W_Interact`))
  ;[1 1 1] Set Visible/UnVisible inscription E
  (`self.EnableInput` (`GameplayStatics.GetPlayerController` 0))
  (bind _output_get (set `self.RangePlayer` true))
  (set `/Game/MiniGames/W_Interact.InteractText` (`self.Interact Text`) _w_interact)
  (`WidgetComponent.SetWidget` _widget _w_interact)
  (`SceneComponent.SetVisibility` _widget _output_get false))

(event `self.InteractionTrigger.OnComponentEndOverlap`
  (params (OverlappedComponent :type "PrimitiveComponent Object Reference") (OtherActor :type "Actor Object Reference") (OtherComp :type "PrimitiveComponent Object Reference") (OtherBodyIndex :type Integer))
  ;[1 1 1] Set Visible/UnVisible inscription E
  (bind _output_get (set `self.RangePlayer` false))
  (`SceneComponent.SetVisibility` (`self.Widget`) _output_get false))

(event `Key|E` :consume false
  (params (Key :type "Key Structure"))
  (bind _returnvalue (`GameplayStatics.GetPlayerController` 0))
  ;[1 1 1] Opening the home screen
  (:`Pressed`
    (if (`self.RangePlayer`)
      (bind _returnvalue_2 (`|CreateWidget` "/Game/Computer/Blueprints/ComputerInterface.ComputerInterface_C" _returnvalue))
      (`UserWidget.AddToViewport` _returnvalue_2 0)
      (`WidgetBlueprintLibrary.SetInputMode_UIOnlyEx` _returnvalue _returnvalue_2)
      (set `PlayerController.bShowMouseCursor` true _returnvalue))))

(fn `UserConstructionScript`)