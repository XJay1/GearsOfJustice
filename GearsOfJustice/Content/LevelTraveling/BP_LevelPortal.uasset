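; BP_LevelPortal is an interactable portal that moves the player between streamed levels.
; A sphere overlap with the base character enables input and shows an interact prompt widget, hidden again on exit.
; Pressing E in range disables pawn input, shows the GameInstance loading screen, starts streaming the target level and teleports the character to the Capsule's transform.
; A fixed delay precedes restoring input, closing the loading screen and unloading the current level.
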(event `self.Sphere.OnComponentBeginOverlap`
  (params (OverlappedComponent :type "PrimitiveComponent Object Reference") (OtherActor :type "Actor Object Reference") (OtherComp :type "PrimitiveComponent Object Reference") (OtherBodyIndex :type Integer) (bFromSweep :type Boolean) (SweepResult :type "HitResult Structure (by ref)"))
  (bind _widget (`self.Widget`))
  (bind _w_interact (`self.W_Interact`))
  ;[0.4417 0.4498 1] Надпись
  (bind _asbp_gojbase_character (cast `/Game/Player/BP_GOJBaseCharacter` OtherActor))
  (set `self.As BP GOJBase Character` _asbp_gojbase_character)
  (`self.EnableInput` (`GameplayStatics.GetPlayerController` 0))
  (bind _output_get (set `self.bIsPlayerInRange` true))
  (set `/Game/MiniGames/W_Interact.InteractText` (`self.Interact Text`) _w_interact)
  (`WidgetComponent.SetWidget` _widget _w_interact)
  (`SceneComponent.SetVisibility` _widget _output_get false))

(event `self.Sphere.OnComponentEndOverlap`
  (params (OverlappedComponent :type "PrimitiveComponent Object Reference") (OtherActor :type "Actor Object Reference") (OtherComp :type "PrimitiveComponent Object Reference") (OtherBodyIndex :type Integer))
  ;[0.4417 0.4498 1] Надпись
  (bind _output_get (set `self.bIsPlayerInRange` false))
  (`SceneComponent.SetVisibility` (`self.Widget`) _output_get false))

(event `Key|E` :consume false
  (params (Key :type "Key Structure"))
  (bind _returnvalue (`GameplayStatics.GetPlayerController` 0))
  (bind _capsule (`self.Capsule`))
  (bind _returnvalue_2 (`Controller.K2_GetPawn` _returnvalue))
  ;[1 1 1] Телепортация на новую локацию
  (:`Pressed`
    (if (`self.bIsPlayerInRange`)
      (`self.DisableInput` _returnvalue_2 _returnvalue)
      (bind _asbp_game_instance (cast `/Game/GameInstance/BP_GameInstance` (`GameplayStatics.GetGameInstance`)))
      (`/Game/GameInstance/BP_GameInstance.ShowLoadingScreen` _asbp_game_instance)
      (`GameplayStatics.LoadStreamLevelBySoftObjectPtr` (`self.LevelToLoad`) true)
      (`self.K2_SetActorLocationAndRotation` (`self.As BP GOJBase Character`) (`SceneComponent.K2_GetComponentLocation` _capsule) (`SceneComponent.K2_GetComponentRotation` _capsule) false false)
      (`KismetSystemLibrary.Delay` 3.0)
      (`self.EnableInput` _returnvalue_2 _returnvalue)
      (`/Game/GameInstance/BP_GameInstance.CloseLoadingScreen` _asbp_game_instance)
      (`GameplayStatics.UnloadStreamLevelBySoftObjectPtr` (`self.CurrentLevel`)))))

(fn `UserConstructionScript`)