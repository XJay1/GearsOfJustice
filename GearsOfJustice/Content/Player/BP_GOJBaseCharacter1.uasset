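; BP_GOJBaseCharacter1 is a player character Blueprint that tracks a Morality value and starts NPC dialogue.
; Upmoral and Downmoral events nudge Morality in small steps within a clamped range, and BeginPlay adds a MoralityWidget to the viewport.
; Holding E sets IsDialog; each press also adds and starts both barman and policeman dialogue components, with no proximity or duplicate check.
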(event `Down moral`
  ;[1 1 1] Изменение морали
  (set `self.Morality` (`KismetMathLibrary.FClamp` (- (`self.Morality`) 0.1) -5.0 5.0)))

(event `Up moral`
  ;[1 1 1] Изменение морали
  (set `self.Morality` (`KismetMathLibrary.FClamp` (+ (`self.Morality`) 0.1) -5.0 5.0)))

(event `Key|E`
  (params (Key :type "Key Structure"))
  ;[1 1 1] Начать диалог
  (:`Pressed`
    (set `self.IsDialog` true)
    (bind _returnvalue (`AddComponent|NODE_AddBarmenDialogComponent-0`))
    (`/Game/NPC/DialogComponent/BarmenDialogComponent.Start` _returnvalue)
    (bind _returnvalue_2 (`AddComponent|NODE_AddPolicmanDialogComponent-0`))
    (`/Game/NPC/DialogComponent/PolicmanDialogComponent.Start` _returnvalue_2))
  (:`Released`
    (set `self.IsDialog` false)))

(event `self.ReceiveBeginPlay`
  (bind _returnvalue (`|CreateWidget` "/Game/NPC/Wiget/MoralityWidget.MoralityWidget_C"))
  (bind _output_get (set `self.MoralityWiget` _returnvalue))
  (`UserWidget.AddToViewport` _output_get 0))

(fn `UserConstructionScript`)