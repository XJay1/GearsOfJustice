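; Player pause component that toggles the pause menu on the Pause input, if the GameInstance reports that pausing is available.
; Opening creates W_PauseMenu at a high Z-order, switches to Game and UI input with a visible cursor, pauses the game and calls CallPauseGame with the widget.
; Closing removes the widget, unpauses and calls CallUnPauseGame, leaving input mode and cursor untouched here.
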(event `InputAction|Pause` :paused true
  (params (Key :type "Key Structure"))
  (bind _returnvalue (`GameplayStatics.GetPlayerController` 0))
  (:`Pressed`
    (bind _isavailable (message `/Game/GameInstance/BPI_LoadingScreen.GetIsAvailablePause` (`GameplayStatics.GetGameInstance`)))
    (if _isavailable
      (if (not (`self.IsPauseMenuOpen`))
        (set `self.IsPauseMenuOpen` true)
        (bind _returnvalue_2 (`|CreateWidget` "/Game/Menu/Blueprint/W_PauseMenu.W_PauseMenu_C" _returnvalue))
        (bind _output_get (set `self.PauseMenuWidget` _returnvalue_2))
        (`self.PauseGame` _output_get)
        (`UserWidget.AddToViewport` _output_get 1000)
        (`WidgetBlueprintLibrary.SetInputMode_GameAndUIEx` _returnvalue _output_get "DoNotLock" false)
        (set `PlayerController.bShowMouseCursor` true _returnvalue)
        (`GameplayStatics.SetGamePaused` true)
        (else
          (set `self.IsPauseMenuOpen` false)
          (`Widget.RemoveFromParent` (`self.PauseMenuWidget`))
          (`GameplayStatics.SetGamePaused` false)
          (`self.UnPauseGame`))))))